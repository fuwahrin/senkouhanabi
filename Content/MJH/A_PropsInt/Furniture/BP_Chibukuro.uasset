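; Furniture prop Blueprint for a Chibukuro cabinet, built from body, side, top and door mesh components, with no active gameplay logic.
; The construction script soft-loads a wood material instance by name through LoadMaterialSoft.
; If the load is valid, it applies that material to every listed part, using slot 1 on Door and slot 0 on the rest, including Door2.
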(fn `UserConstructionScript`
  ;[1 1 1] Load Materials
  (bind (_asmaterial_instance _valid) (`/Game/MJH/A_Arch/Blueprints/MasterBP/BP_HouseMacros.LoadMaterialSoft` (`self.Wood2Mat`) (`self.Wood`))
    (:` `
      (if _valid
        (`PrimitiveComponent.SetMaterial` (`self.lateral2`) 0 _asmaterial_instance)
        (`PrimitiveComponent.SetMaterial` (`self.lateral`) 0 _asmaterial_instance)
        (`PrimitiveComponent.SetMaterial` (`self.top`) 0 _asmaterial_instance)
        (`PrimitiveComponent.SetMaterial` (`self.door2`) 0 _asmaterial_instance)
        (`PrimitiveComponent.SetMaterial` (`self.StaticMesh`) 0 _asmaterial_instance)
        (`PrimitiveComponent.SetMaterial` (`self.door`) 1 _asmaterial_instance)))))
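; BP_Floor_Ext_120 is an architectural floor Blueprint, likely an exterior or extension piece, that configures its static mesh at construction time.
; Its construction script runs ConstructionImpl and then the parent construction script.
; ConstructionImpl loads a mesh from Meshes0 by Type and applies a wood material through LoadMaterialAtIndex using the WoodTable names.
; The event graph holds only disabled stubs, so it adds no runtime logic.
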(fn `ConstructionImpl`
  (bind _staticmesh (`self.StaticMesh`))
  ;[1 1 1] Load Materials
  (`/Game/MJH/A_Arch/Blueprints/MasterBP/BP_HouseMacros.LoadMesh` _staticmesh (`self.Meshes_0`) (`self.Type`)
    (:` `
      (`/Game/MJH/A_Arch/Blueprints/MasterBP/BP_HouseMacros.LoadMaterialAtIndex` _staticmesh (`self.WoodTable`) (`self.Wood`)))))

(fn `UserConstructionScript`
  (`self.ConstructionImpl`)
  (`parent.UserConstructionScript`))
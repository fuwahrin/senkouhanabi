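; BP_Wall_45 is an architectural wall piece, named as a 45-degree variant, that configures its appearance in the Construction Script.
; It loads the mesh for the selected Type, sets slot 0 to a soft-referenced material instance looked up in Type2Mat, then loads wood materials for the WoodToSet names.
; The parent Construction Script runs afterward, and the Event Graph has no active logic.
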(fn `UserConstructionScript`
  (`|ExecutionSequence`
    (:`then_0`
      ;[1 1 1] Load Meshes and Materials
      (`/Game/MJH/A_Arch/Blueprints/MasterBP/BP_HouseMacros.LoadMesh` (`self.StaticMesh`) (`self.Meshes`) (`self.Type`)
        (:` `
          (bind _object (`self.LoadSoftObject` (`BlueprintMapLibrary.Map_Find` (`self.Type2Mat`) (`self.Type`))))
          (bind _asmaterial_instance (cast `MaterialInstance` _object))
          (`PrimitiveComponent.SetMaterial` (`self.StaticMesh`) 0 _asmaterial_instance)
          (`/Game/MJH/A_Arch/Blueprints/MasterBP/BP_HouseMacros.LoadMaterial` (`self.StaticMesh`) (`self.WoodToSet`) (`self.Wood`)))))
    (:`then_1`
      (`parent.UserConstructionScript`))))
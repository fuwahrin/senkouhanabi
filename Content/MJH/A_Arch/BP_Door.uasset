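; BP_Door is a configurable Japanese door actor with shoji and door variants, assembled entirely in the construction script with no active event logic.
; Type picks the base mesh and material, then helper calls load the inner mesh and apply the chosen wood materials.
; Paper can be hidden or offset outside, using either bamboo or washi with a decoration material soft-loaded from a map keyed by ShojiDeco.
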(fn `UserConstructionScript`
  (bind _wood (`self.Wood`))
  (bind _internal (`self.internal`))
  (bind _woodtoset (`self.WoodToSet`))
  (bind _paper (`self.paper`))
  (bind _paper_2 (`self.paper`))
  (bind _staticmesh (`self.StaticMesh`))
  (bind _paper_3 (`self.paper`))
  ;[1 1 1] Load Meshes and Materials
  (`|ExecutionSequence`
    (:`then_0`
      (`|ExecutionSequence`
        (:`then_0`
          (switch `/Game/MJH/A_Arch/Blueprints/Enums/EDoorType` (`self.Type`)
            (:`NewEnumerator0`
              (`StaticMeshComponent.SetStaticMesh` _staticmesh "/Game/MJH/A_Arch/Shoji/Meshes/SM_shoji_base.SM_shoji_base" :!label _label)
              (`PrimitiveComponent.SetMaterial` _staticmesh 0 "/Game/MJH/Materials/Mi_Rails_Set1.Mi_Rails_Set1"))
            (:`NewEnumerator1`
              (goto _label))
            (:`NewEnumerator2`
              (goto _label))
            (:`NewEnumerator3`
              (`StaticMeshComponent.SetStaticMesh` _staticmesh "/Game/MJH/A_Arch/Shoji/Meshes/SM_Door_Base.SM_Door_Base" :!label _label_2)
              (`PrimitiveComponent.SetMaterial` _staticmesh 0 "/Game/MJH/Materials/Mi_DoorBase_Set1.Mi_DoorBase_Set1"))
            (:`NewEnumerator4`
              (goto _label_2))
            (:`NewEnumerator5`
              (goto _label))
            (:`NewEnumerator6`
              (goto _label))
            (:`NewEnumerator7`
              (goto _label))
            (:`NewEnumerator8`
              (goto _label))))
        (:`then_1`
          (`/Game/MJH/A_Arch/Blueprints/MasterBP/BP_HouseMacros.LoadMesh` _internal (`self.Meshes_0`) (`self.Type`)
            (:` `
              (`/Game/MJH/A_Arch/Blueprints/MasterBP/BP_HouseMacros.LoadMaterial` _internal _woodtoset _wood
                (:` `
                  (`/Game/MJH/A_Arch/Blueprints/MasterBP/BP_HouseMacros.LoadMaterial` (`self.StaticMesh`) _woodtoset _wood))))))
        (:`then_2`
          (if (`self.PaperOutside`)
            (`SceneComponent.K2_SetRelativeLocation` (`self.paper`) (-1.6 0.0 0.0) false false)
            (else
              (`SceneComponent.K2_SetRelativeLocation` (`self.paper`) (0.0 0.0 0.0) false false))))
        (:`then_3`
          (if (`|EnumInequality` (`self.Type`) "NewEnumerator8")
            (`StaticMeshComponent.SetStaticMesh` (`self.paper`) "/Game/MJH/A_Arch/Shoji/Meshes/SM_shoji_paper.SM_shoji_paper")
            (`PrimitiveComponent.SetMaterial` _paper_2 0 "/Game/MJH/A_Arch/Shoji/Materials/Mi_washi.Mi_washi")
            (`PrimitiveComponent.SetMaterial` _paper_2 1 "/Game/MJH/A_Arch/Shoji/Materials/Mi_washi.Mi_washi")
            (bind _object (`self.LoadSoftObject` (`BlueprintMapLibrary.Map_Find` (`self.ShojiDeco2Mat`) (`self.ShojiDeco`))))
            (bind _asmaterial_instance (cast `MaterialInstance` _object))
            (`PrimitiveComponent.SetMaterial` _paper 0 _asmaterial_instance)
            (`PrimitiveComponent.SetMaterial` _paper 1 _asmaterial_instance)
            (else
              (`StaticMeshComponent.SetStaticMesh` _paper_3 "/Game/MJH/A_Arch/Shoji/Meshes/SM_shoji_bamboo.SM_shoji_bamboo")
              (`PrimitiveComponent.SetMaterial` _paper_3 0 "/Game/MJH/A_Arch/Shoji/Materials/Mi_shoji_bamboo.Mi_shoji_bamboo"))))))
    (:`then_1`
      (`parent.UserConstructionScript`))
    (:`then_2`
      (`SceneComponent.SetVisibility` (`self.paper`) (`self.HasPaper`) false))))
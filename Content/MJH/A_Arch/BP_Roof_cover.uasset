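; Procedural roof cover actor that lays tile meshes in a straight line along X, capped with onigawara (ornamental end tile) pieces.
; The construction script uses MeshCalc to round the length to a whole number of segments, then stretches each spawned mesh to fill it exactly.
; It moves the back onigawara to the far end, with toggles for top-only cover meshes and onigawara bottom pieces.
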(fn `MeshCalc`
  (params (TotalLength :type "Float (double-precision)") (Size :type "Float (double-precision)"))
  (returns (MeshCount :type Integer) (MeshLength :type "Float (double-precision)"))
  (bind _returnvalue (`KismetMathLibrary.Round` (/ TotalLength Size)))
  (return _returnvalue (/ TotalLength (`KismetMathLibrary.Conv_IntToDouble` _returnvalue))))

(fn `UserConstructionScript`
  (locals (MeshCount :type Integer :default 0) (MeshLength :type "Float (double-precision)" :default 0.0) (CurrDist :type "Float (double-precision)") (tmpLocalTransform :type "Transform Structure") (tmpSize :type "Float (double-precision)" :default 0.0))
  (bind _size_x (`KismetMathLibrary.BreakVector` (`self.Size`)))
  (bind _sm_onigawara_back (`self.SM_onigawara_back`))
  (bind _size_x_2 (`KismetMathLibrary.BreakVector` (`self.Size`)))
  (bind _meshlength (`local.MeshLength`))
  (bind (_meshcount _meshlength_2) (`self.MeshCalc` _size_x_2 (`self.MinSize`)))
  (bind (_relativelocation_x _relativelocation_y _relativelocation_z) (`KismetMathLibrary.BreakVector` (`SceneComponent.RelativeLocation` _sm_onigawara_back)))
  ;[1 1 1] Place roof cover meshes along a straight line
  (set `self.Size` (`KismetMathLibrary.MakeVector` _size_x))
  (`|ExecutionSequence`
    (:`then_0`
      (set `local.MeshLength` _meshlength_2)
      (bind _output_get (set `local.MeshCount` _meshcount))
      (for _index (range _output_get)
        (bind _returnvalue (`AddComponent|NODE_AddStaticMeshComponent-0` :`RelativeTransform` (`KismetMathLibrary.MakeTransform` (`KismetMathLibrary.MakeVector` (* _index _meshlength)) (struct) (`KismetMathLibrary.MakeVector` (/ _meshlength (`self.MinSize`)) 1.0 1.0))))
        ;[1 1 1] Has top mesh only?
        (if (`self.TopOnly`)
          (`StaticMeshComponent.SetStaticMesh` _returnvalue "/Game/MJH/A_Arch/roofs/Type_hongawara/Meshes/SM_roof_cover_top_only.SM_roof_cover_top_only")
          (else
            (`StaticMeshComponent.SetStaticMesh` _returnvalue "/Game/MJH/A_Arch/roofs/Type_hongawara/Meshes/SM_roof_cover.SM_roof_cover")))))
    (:`then_1`
      (`SceneComponent.K2_SetRelativeLocation` _sm_onigawara_back (`KismetMathLibrary.MakeVector` _size_x _relativelocation_y _relativelocation_z) false true))
    (:`then_2`
      (if (`self.OniBottom`)
        (`StaticMeshComponent.SetStaticMesh` (`self.SM_oni_bottom`) "/Game/MJH/A_Arch/roofs/Type_hongawara/Meshes/SM_oni_bottom.SM_oni_bottom")
        (`StaticMeshComponent.SetStaticMesh` (`self.SM_oni_bottom_back`) "/Game/MJH/A_Arch/roofs/Type_hongawara/Meshes/SM_oni_bottom.SM_oni_bottom")
        (else
          (`StaticMeshComponent.SetStaticMesh` (`self.SM_oni_bottom`) null)
          (`StaticMeshComponent.SetStaticMesh` (`self.SM_oni_bottom_back`) null))))))
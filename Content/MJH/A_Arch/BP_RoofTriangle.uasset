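; Construction-script building piece for a triangular hongawara roof section, made of two mesh sides in full or half variants.
; Each side's type selects a material instance via the Type2Mat map; non-default types also load a wood material and scale UVs by the first mesh's world scale.
; The second side is offset by Depth, divided by that scale, to set wall thickness, then the parent construction script runs.
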(fn `UserConstructionScript`
  (bind _triangle_hongawara (`self.triangle_hongawara`))
  (bind _returnvalue_x (`KismetMathLibrary.BreakVector` (`SceneComponent.K2_GetComponentScale` (`self.StaticMesh`))))
  (`|ExecutionSequence`
    (:`then_0`
      ;[1 1 1] Choose meshes
      (if (`self.Half`)
        (`StaticMeshComponent.SetStaticMesh` (`self.StaticMesh`) "/Game/MJH/A_Arch/roofs/Type_hongawara/Meshes/SM_triangle_hongawara_half.SM_triangle_hongawara_half")
        (`StaticMeshComponent.SetStaticMesh` (`self.triangle_hongawara`) "/Game/MJH/A_Arch/roofs/Type_hongawara/Meshes/SM_triangle_hongawara_half_2.SM_triangle_hongawara_half_2")
        (else
          (`StaticMeshComponent.SetStaticMesh` (`self.StaticMesh`) "/Game/MJH/A_Arch/roofs/Type_hongawara/Meshes/SM_triangle_hongawara.SM_triangle_hongawara")
          (`StaticMeshComponent.SetStaticMesh` (`self.triangle_hongawara`) "/Game/MJH/A_Arch/roofs/Type_hongawara/Meshes/SM_triangle_hongawara.SM_triangle_hongawara"))))
    (:`then_1`
      ;[1 1 1] Side A: place and scale meshes, setup parameters for mat. instance
      (if (`|EnumEquality` (`self.TypeA`) "NewEnumerator0")
        (bind _object (`self.LoadSoftObject` (`BlueprintMapLibrary.Map_Find` (`self.Type2Mat`) (`self.TypeA`))))
        (bind _asmaterial_instance (cast `MaterialInstance` _object))
        (`PrimitiveComponent.SetMaterial` (`self.StaticMesh`) 0 _asmaterial_instance)
        (else
          (bind _object_2 (`self.LoadSoftObject` (`BlueprintMapLibrary.Map_Find` (`self.Type2Mat`) (`self.TypeA`))))
          (bind _asmaterial_instance_2 (cast `MaterialInstance` _object_2))
          (`PrimitiveComponent.SetMaterial` (`self.StaticMesh`) 0 _asmaterial_instance_2)
          (`/Game/MJH/A_Arch/Blueprints/MasterBP/BP_HouseMacros.LoadMaterial` (`self.StaticMesh`) (`self.Materials2Set`) (`self.WoodA`)
            (:` `
              (bind _returnvalue (`PrimitiveComponent.CreateDynamicMaterialInstance` (`self.StaticMesh`) 0 null "None"))
              (`MaterialInstanceDynamic.SetScalarParameterValue` _returnvalue "UVMultiplier" _returnvalue_x))))))
    (:`then_2`
      ;[1 1 1] SideB:place and scale meshes, setup parameters for mat. instance
      (if (`|EnumEquality` (`self.TypeB`) "NewEnumerator0")
        (bind _object_3 (`self.LoadSoftObject` (`BlueprintMapLibrary.Map_Find` (`self.Type2Mat`) (`self.TypeB`))))
        (bind _asmaterial_instance_3 (cast `MaterialInstance` _object_3))
        (`PrimitiveComponent.SetMaterial` (`self.triangle_hongawara`) 0 _asmaterial_instance_3)
        (else
          (bind _object_4 (`self.LoadSoftObject` (`BlueprintMapLibrary.Map_Find` (`self.Type2Mat`) (`self.TypeB`))))
          (bind _asmaterial_instance_4 (cast `MaterialInstance` _object_4))
          (`PrimitiveComponent.SetMaterial` (`self.triangle_hongawara`) 0 _asmaterial_instance_4)
          (`/Game/MJH/A_Arch/Blueprints/MasterBP/BP_HouseMacros.LoadMaterial` (`self.triangle_hongawara`) (`self.Materials2Set`) (`self.WoodB`)
            (:` `
              (bind _returnvalue_2 (`PrimitiveComponent.CreateDynamicMaterialInstance` (`self.triangle_hongawara`) 0 null "None"))
              (`MaterialInstanceDynamic.SetScalarParameterValue` _returnvalue_2 "UVMultiplier" _returnvalue_x))))))
    (:`then_3`
      ;[1 1 1] change depth of the wall
      (`SceneComponent.K2_SetRelativeLocation` _triangle_hongawara (`KismetMathLibrary.MakeVector` (.x (`SceneComponent.RelativeLocation` _triangle_hongawara)) (/ (`self.Depth`) _returnvalue_x) (.z (`SceneComponent.RelativeLocation` _triangle_hongawara))) false false))
    (:`then_4`
      (`parent.UserConstructionScript`))))
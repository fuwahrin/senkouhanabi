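; BP_Beam_40 is a modular architectural beam that configures its mesh and wood materials at construction.
; ConstructionImpl resolves Size through FindVariant, loads that variant's mesh, and applies WoodA and WoodB materials to its first two slots.
; Two text components display the Y size as editor helper labels, positioned relative to Size.
; An unwired Loaded guard for skipping construction on level open remains, and the event graph is inactive.
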(fn `ConstructionImpl`
  (bind (_size_x _size_y) (`KismetMathLibrary.BreakVector` (`self.Size`)))
  (bind _txtsizeb (`self.TxtSizeB`))
  (bind _txtsizea (`self.TxtSizeA`))
  (bind (_out _mesh) (`self.FindVariant` (`self.Size`)))
  (bind _returnvalue (`KismetTextLibrary.Conv_DoubleToText` _size_y "HalfToEven" false true 1 324 0 0))
  (`|ExecutionSequence`
    (:`then_0`
      ;[1 1 1] Set the mesh corresponding to size
      (set `self.Size` _out)
      (bind _mesh_2 (`self.LoadMeshF` _mesh))
      (`StaticMeshComponent.SetStaticMesh` (`self.StaticMesh`) _mesh_2)
      ;[1 1 1] Shows helper texts in editor
      (`TextRenderComponent.K2_SetText` _txtsizea _returnvalue)
      (`SceneComponent.K2_SetRelativeLocation` _txtsizea (+ (`self.Size`) (-1.0 -10.0 15.0)) false false)
      (`TextRenderComponent.K2_SetText` _txtsizeb _returnvalue)
      (`SceneComponent.K2_SetRelativeLocation` _txtsizeb (+ (`self.Size`) (21.0 -10.0 15.0)) false false))
    (:`then_1`
      ;[1 1 1] Load materials
      (`/Game/MJH/A_Arch/Blueprints/MasterBP/BP_HouseMacros.LoadMaterialAtIndex` (`self.StaticMesh`) (`self.WoodToSet`) (`self.WoodA`)
        (:` `
          (`/Game/MJH/A_Arch/Blueprints/MasterBP/BP_HouseMacros.LoadMaterialAtIndex` (`self.StaticMesh`) (`self.WoodToSet`) (`self.WoodB`) 1))))))

(fn `UserConstructionScript`
  (`self.ConstructionImpl`)
  (`parent.UserConstructionScript`))
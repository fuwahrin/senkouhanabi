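; Base Blueprint, apparently for modular architecture actors, providing shared helpers for mesh and material setup; its events and construction script do nothing.
; Material helpers rebuild asset names by swapping the "_Set" suffix and load them from MaterialsPath through the Asset Registry.
; Other helpers load soft references, find nearest sizes or Variants, set dynamic material parameters and hide empty mesh components.
; A disconnected construction-script workaround for false lighting-rebuild warnings rounds actor location.
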(fn `FindSize`
  (params (Sizes :type "Array of Float (double-precision) (by ref)") (In :type "Float (double-precision)"))
  (returns (out :type "Float (double-precision)") (index :type Integer))
  (locals (tmpIn :type "Float (double-precision)") (tmpDist :type "Float (double-precision)" :default 100000.0) (tmpSize :type "Float (double-precision)") (tmpIndex :type Integer))
  ;[1 1 1] Finds nearest size in array of sizes
  (set `local.tmpIn` In)
  (for (_array_element _array_index) Sizes
    (bind _returnvalue (`KismetMathLibrary.Abs` (- _array_element (`local.tmpIn`))))
    (if (< _returnvalue (`local.tmpDist`))
      (set `local.tmpDist` _returnvalue)
      (set `local.tmpIndex` _array_index)
      (set `local.tmpSize` _array_element)))
  (return (`local.tmpSize`) (`local.tmpIndex`)))

(fn `FindSizeForType`
  (params (type :type Byte))
  (returns (found :type Boolean) (size :type "Vector Structure"))
  (locals (TmpIn :type Byte) (tmpVariant :type "/Game/MJH/A_Arch/Blueprints/MasterBP/SVariant Structure"))
  ;[1 1 1] Find size for a specified type by searching in Variants array
  (set `local.TmpIn` type)
  (`|ExecutionSequence`
    (:`then_0`
      (for _array_element (`self.Variants`)
        (if (== (`.Type_8_279B9F334093A7155C453C9D212DD10E` (break `/Game/MJH/A_Arch/Blueprints/MasterBP/SVariant` _array_element)) (`local.TmpIn`))
          (return true (break `/Game/MJH/A_Arch/Blueprints/MasterBP/SVariant` _array_element)))))
    (:`then_1`
      (return false (0.0 0.0 0.0)))))

(fn `FindVariant`
  (params (In :type "Vector Structure"))
  (returns (out :type "Vector Structure") (mesh :type "StaticMesh Soft Object Reference") (type :type Byte))
  (locals (TmpIn :type "Vector Structure") (TmpOut :type "Vector Structure") (tmpMesh :type "StaticMesh Soft Object Reference") (tmpDist :type "Float (double-precision)" :default 10000000.0) (tmpVariant :type "/Game/MJH/A_Arch/Blueprints/MasterBP/SVariant Structure"))
  (bind (_tmpvariant_size _tmpvariant_mesh _tmpvariant_type) (break `/Game/MJH/A_Arch/Blueprints/MasterBP/SVariant` (`local.tmpVariant`)))
  ;[1 1 1] Find a mesh from Variants array based on the size input
  (set `local.TmpIn` In)
  (`|ExecutionSequence`
    (:`then_0`
      (for _array_element (`self.Variants`)
        (bind _returnvalue (`KismetMathLibrary.VSizeSquared` (- (break `/Game/MJH/A_Arch/Blueprints/MasterBP/SVariant` _array_element) (`local.TmpIn`))))
        (if (< _returnvalue (`local.tmpDist`))
          (set `local.tmpDist` _returnvalue)
          (set `local.tmpVariant` (make `/Game/MJH/A_Arch/Blueprints/MasterBP/SVariant` (break `/Game/MJH/A_Arch/Blueprints/MasterBP/SVariant` _array_element) (`.Mesh_5_FC99CF2D4A4E658D442249B23434BEE9` (break `/Game/MJH/A_Arch/Blueprints/MasterBP/SVariant` _array_element)) (`.Type_8_279B9F334093A7155C453C9D212DD10E` (break `/Game/MJH/A_Arch/Blueprints/MasterBP/SVariant` _array_element)))))))
    (:`then_1`
      (return _tmpvariant_size _tmpvariant_mesh _tmpvariant_type))))

(fn `HideNullMeshes`
  ;[1 1 1] Sets visibility to false for null static meshes
  (for _array_element (`self.K2_GetComponentsByClass` "/Script/Engine.StaticMeshComponent")
    (`SceneComponent.SetVisibility` _array_element (and (`SceneComponent.bVisible` _array_element) (`KismetSystemLibrary.IsValid` (`StaticMeshComponent.StaticMesh` _array_element))) false)))

(fn `LoadMeshF`
  (params (SoftMesh :type "StaticMesh Soft Object Reference"))
  (returns (Mesh :type "StaticMesh Object Reference") (valid :type Boolean))
  ;[1 1 1] Load mesh from soft object reference
  (if (`KismetSystemLibrary.IsValidSoftObjectReference` SoftMesh)
    ;;[1 1 1] Load object from soft object reference
    (bind _returnvalue (`AssetRegistry.GetAssetByObjectPath` (`AssetRegistryHelpers.GetAssetRegistry`) (`KismetStringLibrary.Conv_StringToName` (`KismetSystemLibrary.Conv_SoftObjectReferenceToString` SoftMesh)) false))
    (bind _asstatic_mesh (cast `StaticMesh` (`AssetRegistryHelpers.GetAsset` _returnvalue))
      (:`then`
        (return _asstatic_mesh (`KismetSystemLibrary.IsValid` _asstatic_mesh)))
      (:`CastFailed`
        (return null false)))
    (else
      (return null false))))

(fn `LoadSoftObject`
  (params (SoftObjectReference :type "Object Soft Object Reference (by ref)"))
  (returns (Object :type "Object Object Reference") (Valid :type Boolean))
  ;[1 1 1] Load object from soft object reference
  (if (`KismetSystemLibrary.IsValidSoftObjectReference` SoftObjectReference)
    (bind _returnvalue (`AssetRegistry.GetAssetByObjectPath` (`AssetRegistryHelpers.GetAssetRegistry`) (`KismetStringLibrary.Conv_StringToName` (`KismetSystemLibrary.Conv_SoftObjectReferenceToString` SoftObjectReference)) false))
    (bind _returnvalue_2 (`AssetRegistryHelpers.GetAsset` _returnvalue))
    (return _returnvalue_2 (`KismetSystemLibrary.IsValid` _returnvalue_2))
    (else
      (return null false))))

(fn `ReplaceMaterial`
  (params (Mesh :type "StaticMeshComponent Object Reference") (Set :type String))
  (for (_array_element _array_index) (`MeshComponent.GetMaterials` Mesh)
    (bind _returnvalue (`KismetStringLibrary.Concat_StrStr` (`KismetStringLibrary.Split` (`KismetSystemLibrary.GetObjectName` _array_element) "_Set" "IgnoreCase" "FromEnd") "_" Set))
    ;[1 1 1] Load material using the name and Materials Path variable
    (bind _returnvalue_2 (`AssetRegistry.GetAssetByObjectPath` (`AssetRegistryHelpers.GetAssetRegistry`) (`KismetStringLibrary.Conv_StringToName` (`KismetStringLibrary.Concat_StrStr` (`self.MaterialsPath`) _returnvalue "." _returnvalue)) false))
    (bind _asmaterial_instance (cast `MaterialInstance` (`AssetRegistryHelpers.GetAsset` _returnvalue_2)))
    (`PrimitiveComponent.SetMaterial` Mesh _array_index _asmaterial_instance)))

(fn `ReplaceMaterialAtIndex`
  (params (Mesh :type "StaticMeshComponent Object Reference") (Set :type String) (Slot :type Integer))
  (bind _returnvalue (`KismetStringLibrary.Concat_StrStr` (`KismetStringLibrary.Split` (`KismetSystemLibrary.GetObjectName` (`|GetArrayItem` (`MeshComponent.GetMaterials` Mesh) Slot)) "_Set" "IgnoreCase" "FromEnd") "_" Set))
  ;[1 1 1] Calculate material name by replacing the "set" suffix, then load the material object from path
  (bind _returnvalue_2 (`AssetRegistry.GetAssetByObjectPath` (`AssetRegistryHelpers.GetAssetRegistry`) (`KismetStringLibrary.Conv_StringToName` (`KismetStringLibrary.Concat_StrStr` (`self.MaterialsPath`) _returnvalue "." _returnvalue)) false))
  ;[1 1 1] Put material instance at specified index
  (bind _asmaterial_instance (cast `MaterialInstance` (`AssetRegistryHelpers.GetAsset` _returnvalue_2)))
  (`PrimitiveComponent.SetMaterial` Mesh Slot _asmaterial_instance))

(fn `ReplaceMaterialSlotName`
  (params (Mesh :type "StaticMeshComponent Object Reference") (Set :type String) (Slot :type Name))
  (bind _staticmesh (`StaticMeshComponent.StaticMesh` Mesh))
  (bind _returnvalue (`StaticMesh.GetMaterialIndex` _staticmesh Slot))
  (bind _returnvalue_2 (`KismetStringLibrary.Concat_StrStr` (`KismetStringLibrary.Split` (`KismetSystemLibrary.GetObjectName` (`StaticMesh.GetMaterial` _staticmesh _returnvalue)) "_Set" "IgnoreCase" "FromEnd") "_" Set))
  ;[1 1 1] Calculate material name by replacing the "set" suffix, then load the material object from path
  (bind _returnvalue_3 (`AssetRegistry.GetAssetByObjectPath` (`AssetRegistryHelpers.GetAssetRegistry`) (`KismetStringLibrary.Conv_StringToName` (`KismetStringLibrary.Concat_StrStr` (`self.MaterialsPath`) _returnvalue_2 "." _returnvalue_2)) false))
  ;[1 1 1] Set material at specified slot
  (bind _asmaterial_instance (cast `MaterialInstance` (`AssetRegistryHelpers.GetAsset` _returnvalue_3)))
  (`PrimitiveComponent.SetMaterial` Mesh _returnvalue _asmaterial_instance))

(fn `SetParameter2Mat`
  (params (Mesh :type "StaticMeshComponent Object Reference") (MaterialIndex :type Integer) (Param :type Name) (Value :type "LinearColor Structure"))
  ;[1 1 1] Sets a parameter in a mat. instance
  (if (and (`KismetSystemLibrary.IsValid` Mesh) (`KismetSystemLibrary.IsValid` (`StaticMeshComponent.StaticMesh` Mesh)))
    (bind _returnvalue (`PrimitiveComponent.CreateDynamicMaterialInstance` Mesh MaterialIndex (`PrimitiveComponent.GetMaterial` Mesh MaterialIndex) "None"))
    (`MaterialInstanceDynamic.SetVectorParameterValue` _returnvalue Param Value)))

(fn `UserConstructionScript`)
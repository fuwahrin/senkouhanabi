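; Tatami mat prop Blueprint that selects its static mesh in the Construction Script.
; The Half flag switches between the full and half mat, and TeahouseSpecial swaps the half mat for a teahouse variant, with no effect on the full mat.
; The parent construction script runs after the mesh is set, and the Event Graph holds only disabled default events.
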(fn `UserConstructionScript`
  (`|ExecutionSequence`
    (:`then_0`
      ;[1 1 1] Load Meshes and Materials
      (if (`self.Half`)
        (`StaticMeshComponent.SetStaticMesh` (`self.StaticMesh`) "/Game/MJH/A_Arch/Tatami/Meshes/SM_Tatami_half.SM_Tatami_half")
        (if (`self.TeahouseSpecial`)
          (`StaticMeshComponent.SetStaticMesh` (`self.StaticMesh`) "/Game/MJH/A_Arch/Tatami/Meshes/SM_Tatami_half_teahouse.SM_Tatami_half_teahouse"))
        (else
          (`StaticMeshComponent.SetStaticMesh` (`self.StaticMesh`) "/Game/MJH/A_Arch/Tatami/Meshes/SM_Tatami.SM_Tatami"))))
    (:`then_1`
      (`parent.UserConstructionScript`))))
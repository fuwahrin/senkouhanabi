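; BP_FLoor is a modular floor/ceiling actor that builds itself in its construction script from a chosen size and materials.
; ContructionImpl converts legacy type-based settings to a size, resolves it through FindVariant, then loads that variant's mesh.
; It labels the dimensions with a TextRender helper and applies soft-loaded floor and ceiling materials from lookup maps to separate slots.
; Event graph nodes are disabled, and the skip-on-level-open check is disconnected.
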(fn `ContructionImpl`
  (bind (_size_x _size_y) (`KismetMathLibrary.BreakVector` (`self.Size`)))
  (bind _textrender (`self.TextRender`))
  (bind (_out _mesh _type) (`self.FindVariant` (`self.Size`)))
  (bind (_found _size) (`self.FindSizeForType` (`self.Type`)))
  (`|ExecutionSequence`
    (:`then_0`
      ;[1 1 1] Conversion from type-based system
      (if (`self.UseOldSystem`)
        (if _found
          (set `self.Size` _size)
          (set `self.UseOldSystem` false))))
    (:`then_1`
      ;[1 1 1] Load mesh by site
      (set `self.Size` _out)
      (set `self.Type` (cast `/Game/MJH/A_Arch/Blueprints/Enums/EFloorType` _type))
      (bind _mesh_2 (`self.LoadMeshF` _mesh))
      ;[1 1 1] Show helper text in editor
      (`StaticMeshComponent.SetStaticMesh` (`self.StaticMesh`) _mesh_2)
      (`TextRenderComponent.K2_SetText` _textrender (`|FormatText` "{x} x {y}" _size_x _size_y))
      (`SceneComponent.K2_SetRelativeLocation` _textrender (+ (`self.Size`) (-10.0 -10.0 1.0)) false false))
    (:`then_2`
      ;[1 1 1] Set floor/ceiling materials
      (bind _object (`self.LoadSoftObject` (`BlueprintMapLibrary.Map_Find` (`self.Floor2Mat`) (`self.FloorMaterial`))))
      (bind _asmaterial_instance (cast `MaterialInstance` _object))
      (`PrimitiveComponent.SetMaterial` (`self.StaticMesh`) 0 _asmaterial_instance))
    (:`then_3`
      (bind _object_2 (`self.LoadSoftObject` (`BlueprintMapLibrary.Map_Find` (`self.Ceiling2Mat`) (`self.CeilingMaterial`))))
      (bind _asmaterial_instance_2 (cast `MaterialInstance` _object_2))
      (`PrimitiveComponent.SetMaterial` (`self.StaticMesh`) 1 _asmaterial_instance_2))))

(fn `UserConstructionScript`
  (`self.ContructionImpl`)
  (`parent.UserConstructionScript`))
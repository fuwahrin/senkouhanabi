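; Modular two-sided wall piece that assembles itself in the construction script from a Half or Full width setting.
; Width selects the frame and wall mesh sets, the Y offset of SideB and a matching placeholder static mesh.
; Sides A and B each choose their meshes by their own type and their frame material by their own wood setting.
; The parent construction script runs after this setup.
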(fn `ConstructionImpl`
  (bind _sideb (`self.SideB`))
  (bind _sideb_2 (`self.SideB`))
  (bind _meshesframe240_0 (`self.MeshesFrame240_0`))
  (bind _frame_a (`self.Frame_A`))
  (bind _frame_a_2 (`self.Frame_A`))
  (bind _frame_b (`self.Frame_B`))
  (bind _frame_b_2 (`self.Frame_B`))
  (bind _meshesframe120_0 (`self.MeshesFrame120_0`))
  (bind _mesheswall120_0 (`self.MeshesWall120_0`))
  (bind _mesheswall240_0 (`self.MeshesWall240_0`))
  (bind (_relativelocation_x _relativelocation_y _relativelocation_z) (`KismetMathLibrary.BreakVector` (`SceneComponent.RelativeLocation` _sideb)))
  (bind (_relativelocation_x_2 _relativelocation_y_2 _relativelocation_z_2) (`KismetMathLibrary.BreakVector` (`SceneComponent.RelativeLocation` _sideb_2)))
  ;[1 1 1] Load Meshes and Materials
  (switch `/Game/MJH/A_Arch/Blueprints/Enums/EWallWidth` (`self.Width`)
    (:`NewEnumerator0`
      (`|ExecutionSequence`
        (:`then_0`
          (`/Game/MJH/A_Arch/Blueprints/MasterBP/BP_HouseMacros.LoadMesh` _frame_a_2 _meshesframe120_0 (`self.TypeA`)
            (:` `
              (`/Game/MJH/A_Arch/Blueprints/MasterBP/BP_HouseMacros.LoadMaterial` _frame_a_2 (`self.WoodToSet`) (`self.WoodA`)
                (:` `
                  (`/Game/MJH/A_Arch/Blueprints/MasterBP/BP_HouseMacros.LoadMesh` _frame_b_2 _meshesframe120_0 (`self.TypeB`)
                    (:` `
                      (`/Game/MJH/A_Arch/Blueprints/MasterBP/BP_HouseMacros.LoadMaterial` _frame_b_2 (`self.WoodToSet`) (`self.WoodB`)))))))))
        (:`then_2`
          (`SceneComponent.K2_SetRelativeLocation` _sideb_2 (`KismetMathLibrary.MakeVector` _relativelocation_x_2 120.0 _relativelocation_z_2) false false)
          (`/Game/MJH/A_Arch/Blueprints/MasterBP/BP_HouseMacros.LoadMesh` (`self.Wall_A`) _mesheswall120_0 (`self.TypeA`)
            (:` `
              (`/Game/MJH/A_Arch/Blueprints/MasterBP/BP_HouseMacros.LoadMesh` (`self.Wall_B`) _mesheswall120_0 (`self.TypeB`)
                (:` `
                  (`StaticMeshComponent.SetStaticMesh` (`self.StaticMesh`) "/Game/MJH/A_Arch/Walls/Placeholders/SM_placeholders_p100x80.SM_placeholders_p100x80"))))))))
    (:`NewEnumerator1`
      (`|ExecutionSequence`
        (:`then_0`
          (`/Game/MJH/A_Arch/Blueprints/MasterBP/BP_HouseMacros.LoadMesh` _frame_a _meshesframe240_0 (`self.TypeA`)
            (:` `
              (`/Game/MJH/A_Arch/Blueprints/MasterBP/BP_HouseMacros.LoadMaterial` _frame_a (`self.WoodToSet`) (`self.WoodA`)
                (:` `
                  (`/Game/MJH/A_Arch/Blueprints/MasterBP/BP_HouseMacros.LoadMesh` _frame_b _meshesframe240_0 (`self.TypeB`)
                    (:` `
                      (`/Game/MJH/A_Arch/Blueprints/MasterBP/BP_HouseMacros.LoadMaterial` _frame_b (`self.WoodToSet`) (`self.WoodB`)))))))))
        (:`then_2`
          (`SceneComponent.K2_SetRelativeLocation` _sideb (`KismetMathLibrary.MakeVector` _relativelocation_x 240.0 _relativelocation_z) false false)
          (`/Game/MJH/A_Arch/Blueprints/MasterBP/BP_HouseMacros.LoadMesh` (`self.Wall_A`) _mesheswall240_0 (`self.TypeA`)
            (:` `
              (`/Game/MJH/A_Arch/Blueprints/MasterBP/BP_HouseMacros.LoadMesh` (`self.Wall_B`) _mesheswall240_0 (`self.TypeB`)
                (:` `
                  (`StaticMeshComponent.SetStaticMesh` (`self.StaticMesh`) "/Game/MJH/A_Arch/Walls/Placeholders/SM_placeholders_p220x80.SM_placeholders_p220x80"))))))))))

(fn `UserConstructionScript`
  (`self.ConstructionImpl`)
  (`parent.UserConstructionScript`))
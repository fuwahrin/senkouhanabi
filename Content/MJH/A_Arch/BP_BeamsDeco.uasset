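; BP_BeamsDeco is a decorative beam actor that builds a row of evenly spaced beams in its construction script.
; Length, Wood, Interval and Width options look up mesh, material, spacing and span in maps.
; Instanced static mesh copies are placed along local X, leaving both ends of the span empty.
; An older per-component version is left disconnected, and RoundPosition, though called per instance, does nothing because its snapping logic is unwired.
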(fn `RoundPosition`
  (params (InstMesh :type "InstancedStaticMeshComponent Object Reference")))

(fn `UserConstructionScript`
  (locals (tmpMesh :type "StaticMesh Object Reference") (Width_cm :type "Float (double-precision)") (Int_cm :type "Float (double-precision)") (MeshQut :type Integer :default 0) (MatName :type String))
  (bind _instancedstaticmesh (`self.InstancedStaticMesh`))
  (bind _instancedstaticmesh_2 (`self.InstancedStaticMesh`))
  (`|ExecutionSequence`
    (:`then_0`
      (bind (_mesh _valid) (`self.LoadMeshF` (`BlueprintMapLibrary.Map_Find` (`self.Meshes_0`) (`self.Length`))))
      (if _valid
        (bind _output_get (set `local.tmpMesh` _mesh))
        (`StaticMeshComponent.SetStaticMesh` _instancedstaticmesh _output_get)
        ;[1 1 1] Set Materials
        (set `local.MatName` (`BlueprintMapLibrary.Map_Find` (`self.MaterialMap`) (`self.Wood`)))
        (`self.ReplaceMaterial` _instancedstaticmesh (`local.MatName`))
        (set `local.Int_cm` (`BlueprintMapLibrary.Map_Find` (`self.Int`) (`self.Interval`)))))
    (:`then_1`
      (set `local.Width_cm` (`BlueprintMapLibrary.Map_Find` (`self.WidthMap`) (`self.Width`)))
      (if (> (`local.Int_cm`) 0.0)
        (set `local.MeshQut` (- (`KismetMathLibrary.Round` (/ (`local.Width_cm`) (`local.Int_cm`))) 2))
        ;[1 1 1] Place instanced static meshes
        (for _index (range (+ (`local.MeshQut`) 1))
          (`InstancedStaticMeshComponent.AddInstance` _instancedstaticmesh_2 (`KismetMathLibrary.MakeTransform` (`KismetMathLibrary.MakeVector` (* (+ _index 1) (`local.Int_cm`)))))
          (`self.RoundPosition` _instancedstaticmesh_2))))
    (:`then_2`
      (`parent.UserConstructionScript`))))
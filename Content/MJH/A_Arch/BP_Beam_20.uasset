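; BP_Beam_20 is an architectural beam actor that builds itself in the construction script, with no active runtime logic.
; It snaps Size to a matching variant, then loads that mesh and applies two wood materials by slot name.
; A legacy flag converts old type-based instances to the size-based system.
; Two text renders display the Y size as editor helpers, and the skip-on-level-load guard is disconnected.
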(fn `ConstructionImpl`
  (bind _staticmesh (`self.StaticMesh`))
  (bind (_size_x _size_y) (`KismetMathLibrary.BreakVector` (`self.Size`)))
  (bind _textrender2 (`self.TextRender2`))
  (bind _textrender3 (`self.TextRender3`))
  (bind (_out _mesh _type) (`self.FindVariant` (`self.Size`)))
  (bind (_found _size) (`self.FindSizeForType` (`self.Type`)))
  (bind _result (`|FormatText` "{y}" _size_y))
  (`|ExecutionSequence`
    (:`then_0`
      ;[1 1 1] Conversion from type-based to size based system
      (if (`self.UseOldSystem`)
        (if _found
          (set `self.Size` _size)
          (set `self.UseOldSystem` false))))
    (:`then_1`
      ;[1 1 1] Find Variant mesh based on size
      (set `self.Size` _out)
      (set `self.Type` (cast `/Game/MJH/A_Arch/Blueprints/Enums/ERailUpType` _type))
      (bind _mesh_2 (`self.LoadMeshF` _mesh))
      (`StaticMeshComponent.SetStaticMesh` (`self.StaticMesh`) _mesh_2)
      ;[1 1 1] Helper texts for editor
      (`TextRenderComponent.K2_SetText` _textrender2 _result)
      (`SceneComponent.K2_SetRelativeLocation` _textrender2 (+ (`self.Size`) (1.0 -20.0 -5.0)) false false)
      (`TextRenderComponent.K2_SetText` _textrender3 _result)
      (`SceneComponent.K2_SetRelativeLocation` _textrender3 (+ (`self.Size`) (-21.0 -20.0 -5.0)) false false))
    (:`then_2`
      ;[1 1 1] Set Materials
      (`/Game/MJH/A_Arch/Blueprints/MasterBP/BP_HouseMacros.LoadMaterialAtSlot` _staticmesh (`self.WoodToSet`) (`self.WoodA`) "MatA"
        (:` `
          (`/Game/MJH/A_Arch/Blueprints/MasterBP/BP_HouseMacros.LoadMaterialAtSlot` _staticmesh (`self.WoodToSet`) (`self.WoodB`) "MatB"))))))

(fn `UserConstructionScript`
  (`self.ConstructionImpl`)
  (`parent.UserConstructionScript`))
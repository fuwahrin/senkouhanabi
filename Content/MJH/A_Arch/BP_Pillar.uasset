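; Architectural pillar actor that picks its mesh from a requested size and configures itself in the construction script.
; ConstructionImpl first converts old type-based instances to size-based, then snaps Size and Type to the found variant and loads its mesh.
; It then applies wood materials to two slots and places two editor helper texts showing the dimensions.
; The event graph is unused, and the skip-on-level-open check is disconnected.
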(fn `ConstructionImpl`
  (bind (_size_x _size_y _size_z) (`KismetMathLibrary.BreakVector` (`self.Size`)))
  (bind _txtsizea (`self.TxtSizeA`))
  (bind _txtsizeb (`self.TxtSizeB`))
  (bind (_out _mesh _type) (`self.FindVariant` (`self.Size`)))
  (bind (_found _size) (`self.FindSizeForType` (`self.Type`)))
  (bind _result (`|FormatText` "{z} x {y}" _size_z _size_y))
  (`|ExecutionSequence`
    (:`then_0`
      ;[1 1 1] Conversion from type based to size based system
      (if (`self.UseOldSystem`)
        (if _found
          (set `self.Size` _size)
          (set `self.UseOldSystem` false))))
    (:`then_1`
      ;[1 1 1] Find mesh by size
      (set `self.Size` _out)
      (set `self.Type` (cast `/Game/MJH/A_Arch/Blueprints/Enums/EPillarType` _type))
      (bind _mesh_2 (`self.LoadMeshF` _mesh))
      (`StaticMeshComponent.SetStaticMesh` (`self.StaticMesh`) _mesh_2)
      ;[1 1 1] Setup materials
      (`/Game/MJH/A_Arch/Blueprints/MasterBP/BP_HouseMacros.LoadMaterialAtSlot` self (`self.StaticMesh`) (`self.WoodToSet`) (`self.WoodA`) "MatA"
        (:` `
          (`/Game/MJH/A_Arch/Blueprints/MasterBP/BP_HouseMacros.LoadMaterialAtSlot` self (`self.StaticMesh`) (`self.WoodToSet`) (`self.WoodB`) "MatB"
            (:` `
              ;[1 1 1] Show helper text in editor
              (`TextRenderComponent.K2_SetText` _txtsizea _result)
              (`SceneComponent.K2_SetRelativeLocation` _txtsizea (+ (`self.Size`) (21.0 0.0 -15.0)) false false)
              (`TextRenderComponent.K2_SetText` _txtsizeb _result)
              (`SceneComponent.K2_SetRelativeLocation` _txtsizeb (+ (`self.Size`) (-1.0 -10.0 -15.0)) false false))))))))

(fn `UserConstructionScript`
  (`self.ConstructionImpl`)
  (`parent.UserConstructionScript`))
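; Modular two-sided wall Blueprint that assembles itself in the construction script from width, type, window and wood settings.
; Width selects the 2400 or 1200 mesh sets, moves SideB to a matching Y offset and swaps the placeholder mesh.
; Sides A and B each load their own frame mesh, wood material and wall or window mesh, with IsWindow shared by both.
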(fn `ConstructionImpl`
  (bind _mesheswindow120_0 (`self.MeshesWindow120_0`))
  (bind _sideb (`self.SideB`))
  (bind _sideb_2 (`self.SideB`))
  (bind _frame_a (`self.Frame_A`))
  (bind _frame_b (`self.Frame_B`))
  (bind _is_window (`self.Is Window`))
  (bind _frame_b_2 (`self.Frame_B`))
  (bind _frame_a_2 (`self.Frame_A`))
  (bind _mesheswall120_0 (`self.MeshesWall120_0`))
  (bind (_relativelocation_x _relativelocation_y _relativelocation_z) (`KismetMathLibrary.BreakVector` (`SceneComponent.RelativeLocation` _sideb_2)))
  (bind (_relativelocation_x_2 _relativelocation_y_2 _relativelocation_z_2) (`KismetMathLibrary.BreakVector` (`SceneComponent.RelativeLocation` _sideb)))
  ;[1 1 1] Load Meshes and Materials
  (if (`|EnumEquality` (`self.Width`) "NewEnumerator1")
    (`|ExecutionSequence`
      (:`then_0`
        (`/Game/MJH/A_Arch/Blueprints/MasterBP/BP_HouseMacros.LoadMesh` self _frame_a (`self.MeshesFrame240_0`) (`self.TypeA`)
          (:` `
            (`/Game/MJH/A_Arch/Blueprints/MasterBP/BP_HouseMacros.LoadMaterial` self _frame_a (`self.WoodToSet`) (`self.WoodA`)
              (:` `
                (`/Game/MJH/A_Arch/Blueprints/MasterBP/BP_HouseMacros.LoadMesh` self _frame_b_2 (`self.MeshesFrame240_0`) (`self.TypeB`)
                  (:` `
                    (`/Game/MJH/A_Arch/Blueprints/MasterBP/BP_HouseMacros.LoadMaterial` self _frame_b_2 (`self.WoodToSet`) (`self.WoodB`)))))))))
      (:`then_1`
        (`SceneComponent.K2_SetRelativeLocation` _sideb (`KismetMathLibrary.MakeVector` _relativelocation_x_2 240.0 _relativelocation_z_2) false false)
        (`/Game/MJH/A_Arch/Blueprints/MasterBP/BP_HouseMacros.LoadMeshSelect` self (`self.Wall_A`) (`self.Is Window`) (`self.MeshesWindow240_0`) (`self.MeshesWall240_0`) (`self.TypeA`)
          (:`   `
            (`/Game/MJH/A_Arch/Blueprints/MasterBP/BP_HouseMacros.LoadMeshSelect` self (`self.Wall_B`) (`self.Is Window`) (`self.MeshesWindow240_0`) (`self.MeshesWall240_0`) (`self.TypeB`)
              (:`   `
                (`StaticMeshComponent.SetStaticMesh` (`self.StaticMesh`) "/Game/MJH/A_Arch/Walls/Placeholders/SM_placeholders_p220x240.SM_placeholders_p220x240")))))))
    (else
      (`|ExecutionSequence`
        (:`then_0`
          (`/Game/MJH/A_Arch/Blueprints/MasterBP/BP_HouseMacros.LoadMesh` self _frame_a_2 (`self.MeshesFrame120_0`) (`self.TypeA`)
            (:` `
              (`/Game/MJH/A_Arch/Blueprints/MasterBP/BP_HouseMacros.LoadMaterial` self _frame_a_2 (`self.WoodToSet`) (`self.WoodA`)
                (:` `
                  (`/Game/MJH/A_Arch/Blueprints/MasterBP/BP_HouseMacros.LoadMesh` self _frame_b (`self.MeshesFrame120_0`) (`self.TypeB`)
                    (:` `
                      (`/Game/MJH/A_Arch/Blueprints/MasterBP/BP_HouseMacros.LoadMaterial` self _frame_b (`self.WoodToSet`) (`self.WoodB`)))))))))
        (:`then_1`
          (`SceneComponent.K2_SetRelativeLocation` _sideb_2 (`KismetMathLibrary.MakeVector` _relativelocation_x 120.0 _relativelocation_z) false false)
          (`/Game/MJH/A_Arch/Blueprints/MasterBP/BP_HouseMacros.LoadMeshSelect` self (`self.Wall_A`) _is_window _mesheswindow120_0 _mesheswall120_0 (`self.TypeA`)
            (:`   `
              (`/Game/MJH/A_Arch/Blueprints/MasterBP/BP_HouseMacros.LoadMeshSelect` self (`self.Wall_B`) _is_window _mesheswindow120_0 _mesheswall120_0 (`self.TypeB`)
                (:`   `
                  (`StaticMeshComponent.SetStaticMesh` (`self.StaticMesh`) "/Game/MJH/A_Arch/Walls/Placeholders/SM_placeholders_p100x240.SM_placeholders_p100x240"))))))))))

(fn `UserConstructionScript`
  (`self.ConstructionImpl`)
  (`parent.UserConstructionScript`))
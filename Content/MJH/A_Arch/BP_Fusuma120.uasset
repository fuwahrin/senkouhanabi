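; Fusuma (Japanese sliding panel) Blueprint that sets the decoration material on each of its two sides in the construction script, then runs the parent's script.
; SetDeco joins a decoration name and a position suffix from lookup maps, then resolves that material instance by path through the Asset Registry.
; One decoration option skips the lookup and applies a paper material; each side fills its own static mesh slot.
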(fn `SetDeco`
  (params (Deco :type "/Game/MJH/A_Arch/Blueprints/Enums/EFusumaDeco Enum" :default "NewEnumerator4") (Position :type "/Game/MJH/A_Arch/Blueprints/Enums/EFusumaPosition Enum" :default "NewEnumerator0") (SlotIndex :type Integer))
  (locals (locDeco :type "/Game/MJH/A_Arch/Blueprints/Enums/EFusumaDeco Enum" :default "NewEnumerator4") (tmpString :type String))
  (bind _tmpstring (`local.tmpString`))
  (bind (_value _returnvalue) (`BlueprintMapLibrary.Map_Find` (`self.PosToString`) Position))
  (bind (_value_2 _returnvalue_2) (`BlueprintMapLibrary.Map_Find` (`self.MaterialMap`) (`local.locDeco`)))
  (set `local.locDeco` Deco)
  (if (`|EnumInequality` (`local.locDeco`) "NewEnumerator4")
    (if _returnvalue_2
      (set `local.tmpString` _value_2)
      (if _returnvalue
        (set `local.tmpString` (`KismetStringLibrary.Concat_StrStr` (`local.tmpString`) _value))
        (bind _returnvalue_3 (`AssetRegistry.GetAssetByObjectPath` (`AssetRegistryHelpers.GetAssetRegistry`) (`KismetStringLibrary.Conv_StringToName` (`KismetStringLibrary.Concat_StrStr` (`self.MaterialsPath`) _tmpstring "." _tmpstring)) false))
        (bind _asmaterial_instance (cast `MaterialInstance` (`AssetRegistryHelpers.GetAsset` _returnvalue_3)))
        (`PrimitiveComponent.SetMaterial` (`self.StaticMesh`) SlotIndex _asmaterial_instance)))
    (else
      (`PrimitiveComponent.SetMaterial` (`self.StaticMesh`) SlotIndex "/Game/MJH/Materials/Mi_paper.Mi_paper"))))

(fn `UserConstructionScript`
  (`|ExecutionSequence`
    (:`then_0`
      ;[1 1 1] Load Materials
      (`self.SetDeco` (`self.SideA_Deco`) (`self.SideA_Position`))
      (`self.SetDeco` (`self.SideB_Deco`) (`self.SideB_Position`) 1))
    (:`then_1`
      (`parent.UserConstructionScript`))))
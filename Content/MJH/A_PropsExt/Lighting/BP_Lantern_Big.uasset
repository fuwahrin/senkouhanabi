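; BP_Lantern_Big is a large lantern prop with a light that responds to a light-down event from the player controller.
; Construction sets the optional cover, light color and a dynamic material with color, emissive and a text texture looked up from LanternText via the Asset Registry.
; On BeginPlay it binds LightDown to BP_FireSparkMusicGamevController's event, which plays a timeline driving the light's intensity.
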(event `self.ReceiveBeginPlay`
  (bind _asbp_fire_spark_music_gamev_controller (cast `/Game/Developers/fuwarrin/Collections/FireSpark/BP_FireSparkMusicGamevController` (`GameplayStatics.GetPlayerController` 0)))
  (add `/Game/Developers/fuwarrin/Collections/FireSpark/BP_FireSparkMusicGamevController.LightDonwEvent` _asbp_fire_spark_music_gamev_controller (delegate `LightDown`)))

(event `LightDown`
  (bind (_direction _lightdown) (`Timeline|タイムライン_0` :!via `PlayFromStart`)
    (:`Update`
      (`LightComponent.SetIntensity` (`self.LightComponent0`) _lightdown))))

(fn `UserConstructionScript`
  (bind _color (`self.Color`))
  (bind _materialinst (`self.MaterialInst`))
  (bind _lanterncover (`self.LanternCover`))
  ;[1 1 1] Set parameters for material instance
  (`|ExecutionSequence`
    (:`then_0`
      ;[1 1 1] Setup cover
      (if (`self.Cover?`)
        (`StaticMeshComponent.SetStaticMesh` _lanterncover "/Game/MJH/A_PropsExt/Lighting/Meshes/SM_Lantern_Big_cover.SM_Lantern_Big_cover")
        (else
          (`StaticMeshComponent.SetStaticMesh` _lanterncover null))))
    (:`then_1`
      (bind _returnvalue (`PrimitiveComponent.CreateDynamicMaterialInstance` (`self.Lantern`) 0 "/Game/MJH/A_PropsExt/Lighting/Materials/Mi_Lantern_Big.Mi_Lantern_Big" "None"))
      (set `self.MaterialInst` _returnvalue)
      (`MaterialInstanceDynamic.SetVectorParameterValue` _materialinst "LanternColor" _color)
      (`MaterialInstanceDynamic.SetVectorParameterValue` _materialinst "EmissiveCol" _color)
      ;[1 1 1] Load object from soft object reference
      (bind _returnvalue_2 (`AssetRegistry.GetAssetByObjectPath` (`AssetRegistryHelpers.GetAssetRegistry`) (`KismetStringLibrary.Conv_StringToName` (`KismetSystemLibrary.Conv_SoftObjectReferenceToString` (`BlueprintMapLibrary.Map_Find` (`self.Text2Texture`) (`self.LanternText`)))) false))
      (bind _astexture_2d (cast `Texture2D` (`AssetRegistryHelpers.GetAsset` _returnvalue_2)))
      (`MaterialInstanceDynamic.SetTextureParameterValue` (`self.MaterialInst`) "additionalTexture" _astexture_2d))
    (:`then_2`
      ;;[1 1 1] Set light color
      (`LightComponent.SetLightColor` (`self.LightComponent0`) (`self.LightColor`) true))))